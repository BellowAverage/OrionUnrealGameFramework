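; BP_OrionActor is an actor with an optional looping self-rotation of its SMRoot component.
; The OrionActorSelfRotation event, not called within this graph, plays a timeline that lerps SMRoot's world rotation toward a full 360-degree turn and re-triggers itself on finish.
; An unconnected piston template sketches vertical oscillation through OrionOscillation but never runs; BeginPlay and the construction script are empty.
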(event Custom|OrionActorSelfRotation
  ;[0.15 0.15 0.15 0.5] Enable Self Rotation
  (bind _rotation (Timeline|OrionActorSelfRotationTimeline PlayFromStart)
    (:Update
      (Transformation|SetWorldRotation (Variables|Default|GetSM_Root) (Math|Rotator|Lerp(Rotator) "0, 0, 0" "0.000000,360.000000,0.000000" _rotation) false false))
    (:Finished
      (CallFunction|OrionActorSelfRotation))))

(event EventBeginPlay)

(event Collision|EventActorBeginOverlap
  (params (OtherActor :type Actor%20Object%20Reference)))

(event EventTick
  (params (DeltaSeconds :type Float%20%28single-precision%29)))

(fn ConstructionScript)