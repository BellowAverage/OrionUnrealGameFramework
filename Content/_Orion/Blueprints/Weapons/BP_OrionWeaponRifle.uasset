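; Rifle weapon Blueprint for Orion that configures how its owning BP_XChara carries it and attacks at long range.
; On BeginPlay it casts its owner to BP_XChara and passes back and hand attach transforms, right-hand use, spawn offset and long-range attack timing through GetAttachBackTransformation.
; The construction script applies the hand attach offsets to the OrionWeapon component's relative transform.
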(event EventBeginPlay
  (|CallParentFunction)
  (bind _asbp_xchara (Utilities|Casting|CastToBP_XChara (Components|GetOwner)))
  (Default|GetAttachBackTransformation _asbp_xchara (Math|Transform|MakeTransform (Variables|Default|GetBackAttachLocationOffset) (Variables|Default|GetBackAttachRotationOffset) "1.500000,1.500000,1.500000") (Math|Transform|MakeTransform (Variables|Default|GetHandAttachLocationOffset) (Variables|Default|GetHandAttachRotationOffset)) true 5e+01 (Variables|Default|GetAttackFrequencyLongRange) (Variables|Default|GetAttackTriggerTimeLongRange)))

(event Collision|EventActorBeginOverlap
  (params (OtherActor :type Actor%20Object%20Reference))
  (|CallParentFunction OtherActor) ; This node is disabled and will not be called.\nDrag off pins to build functionality.
)

(event EventTick
  (params (DeltaSeconds :type Float%20%28single-precision%29))
  (|CallParentFunction DeltaSeconds))

(fn ConstructionScript
  (|CallParentFunction)
  (Transformation|SetRelativeTransform (Variables|Default|GetOrionWeapon) (Math|Transform|MakeTransform (Variables|Default|GetHandAttachLocationOffset) (Variables|Default|GetHandAttachRotationOffset)) false false))